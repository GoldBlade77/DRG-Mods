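; Component that converts its owning Loot Bug into a red sugar variant with a healing-crystal look and red sugar loot.
; On BeginPlay it swaps the mesh material, raises the net update frequency, sets the chunk value range and calls UpdateBug.
; UpdateBug stores and applies walk speed and scale, then refills the loot list with red sugar chunks on the authority only.
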(event `self.ReceiveBeginPlay`
  (bind _returnvalue (`self.GetOwner`))
  (`/Engine/EditorBlueprintResources/StandardMacros.IsValid` _returnvalue
    (:`Is Valid`
      (bind _asene_loot_bug (cast `/Game/Critters/LootBug/ENE_LootBug` _returnvalue))
      (set `self.LootBug` _asene_loot_bug)
      (set `Actor.NetUpdateFrequency` 1000.0 (`self.LootBug`))
      (bind _returnvalue_2 (`KismetMaterialLibrary.CreateDynamicMaterialInstance` "/Game/Art/Environments/Crystals/M_Crystal_Healing.M_Crystal_Healing"))
      (`PrimitiveComponent.SetMaterial` (`DeepPathfinderCharacter.Mesh` (`self.LootBug`)) 0 _returnvalue_2)
      (set `/Game/Critters/LootBug/ENE_LootBug.ChunkValueRange` (`self.ChunkValueRange`) (`self.LootBug`))
      (`self.UpdateBug` (`self.WalkSpeed`) (`self.ChunkCount`) (`self.BugScale`)))))

(event `UpdateBug`
  (params (WalkSpeed :type "Float (double-precision)") (ChunkCount :type Integer) (BugScale :type "Float (double-precision)"))
  (bind _walkspeed (`self.WalkSpeed`))
  (bind _pathfindermovement (`DeepPathfinderCharacter.PathfinderMovement` (`self.LootBug`)))
  (set `self.WalkSpeed` WalkSpeed)
  (set `self.ChunkCount` ChunkCount)
  (set `self.BugScale` BugScale)
  (`DeepPathfinderMovement.SetMaxSpeed` _pathfindermovement _walkspeed)
  (set `DeepPathfinderMovement.MaxAcceleration` _walkspeed _pathfindermovement)
  (`Actor.SetActorScale3D` (`self.LootBug`) (`KismetMathLibrary.Conv_DoubleToVector` (`self.BugScale`)))
  (if (`Actor.HasAuthority` (`self.LootBug`))
    (`KismetArrayLibrary.Array_Clear` (`/Game/Critters/LootBug/ENE_LootBug.Loot` (`self.LootBug`)))
    (for _ (range 1 (+ (`self.ChunkCount`) 1))
      (`KismetArrayLibrary.Array_Add` (`/Game/Critters/LootBug/ENE_LootBug.Loot` (`self.LootBug`)) "/Game/GameElements/Resources/Carved/RedSugar/RES_CARVED_RedSugar.RES_CARVED_RedSugar"))))