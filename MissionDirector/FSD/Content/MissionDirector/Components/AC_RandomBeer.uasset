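; AC_RandomBeer is an actor component that gives the owning player character a random beer effect when play begins.
; It picks a random class from BeerEffects, adds it to the player as a component and sets that effect's duration to a fixed value.
; After a delay of that duration, it clears the player's intoxication through the IntoxicationComponent.
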(event `self.ReceiveBeginPlay`
  (bind _asbp_player_character (cast `/Game/Character/BP_PlayerCharacter` (`self.GetOwner`)))
  (bind _output_get (set `self.Player` _asbp_player_character))
  (bind _returnvalue (`|AddComponentByClass` _output_get (`KismetArrayLibrary.Array_Random` (`self.BeerEffects`))))
  (bind _output_get_2 (set `DrinkEffectComponent.BeerEffectDurationSeconds` 15.0 _returnvalue))
  (`KismetSystemLibrary.Delay` _output_get_2)
  (`CharacterIntoxicationComponent.ClearIntoxication` (`PlayerCharacter.IntoxicationComponent` (`self.Player`))))