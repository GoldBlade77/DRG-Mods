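; Spawn menu actor component that temporarily makes the owning player character drunk.
; Its MakeDrunk event drives the player's IntoxicationComponent with a high lerping intoxication percent and the Intoxicated state, then clears it after a fixed delay.
; An IsDrunk flag blocks retriggering during the effect; it is set before the owner cast, so it stays set if that cast fails.
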(event `MakeDrunk`
  (if (not (`self.IsDrunk`))
    (set `self.IsDrunk` true)
    (bind _asbp_player_character (cast `/Game/Character/BP_PlayerCharacter` (`self.GetOwner`)))
    (bind _output_get (set `self.Player` _asbp_player_character))
    (bind _intoxicationcomponent (`PlayerCharacter.IntoxicationComponent` _output_get))
    (set `CharacterIntoxicationComponent.IntoxicationPercent` (make `LerpingPercent` 0.8) _intoxicationcomponent)
    (set `CharacterIntoxicationComponent.CurrentState` "Intoxicated" _intoxicationcomponent)
    (`KismetSystemLibrary.Delay` 15.0)
    (`CharacterIntoxicationComponent.ClearIntoxication` (`PlayerCharacter.IntoxicationComponent` (`self.Player`)))
    (set `self.IsDrunk` false)))