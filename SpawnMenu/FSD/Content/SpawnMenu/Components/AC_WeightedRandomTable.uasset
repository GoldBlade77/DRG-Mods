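; AC_WeightedRandomTable is a spawn menu component that picks a random actor entry from a weighted table.
; RandomActorWithWeight totals the values of the ActorWeightTable map and rolls a float between zero and that sum.
; It walks the keys, subtracting each weight from the roll until one covers it, then returns that key with a success flag, or false if none matches.
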(fn `RandomActorWithWeight`
  (returns (ReturnValue :type Boolean) (RandomActor :type "Actor Class Reference"))
  (locals (SumOfAllWeights :type "Float (double-precision)") (RandomValueInSum :type "Float (double-precision)"))
  (bind _values (`BlueprintMapLibrary.Map_Values` (`self.ActorWeightTable`)))
  (for _array_element _values
    (set `local.SumOfAllWeights` (+ _array_element (`local.SumOfAllWeights`))))
  (set `local.RandomValueInSum` (`KismetMathLibrary.RandomFloatInRange` 0.0 (`local.SumOfAllWeights`)))
  (bind _keys (`BlueprintMapLibrary.Map_Keys` (`self.ActorWeightTable`)))
  (for _array_element_2 _keys
    (bind _value (`BlueprintMapLibrary.Map_Find` (`self.ActorWeightTable`) _array_element_2))
    (if (<= (`local.RandomValueInSum`) _value)
      (return true _array_element_2) ; Found, return actor.
      (else
        (set `local.RandomValueInSum` (- (`local.RandomValueInSum`) _value)))))
  (return false null) ; Nothing found, return null.
)