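; BP_ArchitectMode is an in-game director mode for placing and editing decorations with a free-fly camera.
; Starting it takes view and input from the player's pawn, enables a skylight, spawns a transform gizmo and shows the ArchtectHud.
; Placement mode moves a data-driven marker along a cursor trace aligned to surface normals.
; Edit mode selects Decoration_Base actors for gizmo transforms, deletion or duplication.
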(event `self.ReceiveBeginPlay`
  (set `self.Player` (`/Game/Architect/Libraries/ArchitectFunctions.GetLocalPlayer`))
  (`self.ChangeMode` "NewEnumerator0")
  (bind _returnvalue (`|CreateWidget` "/Game/Architect/Architect/HUD/ArchtectHud.ArchtectHud_C"))
  (set `self.Hud` _returnvalue))

(event `Key|W`
  (params (Key :type "Key Structure"))
  (:`Pressed`
    (set `self.Is Forward Pressed` true))
  (:`Released`
    (set `self.Is Forward Pressed` false)))

(event `Key|RightMouseButton` :consume false
  (params (Key :type "Key Structure"))
  (:`Pressed`
    (set `self.Is RM Down` true)
    (`self.HideMouseCursor`)
    (`WidgetBlueprintLibrary.SetInputMode_GameOnly` (`self.Player`))
    (`self.SetActorHiddenInGame` (`self.CurrentMarker`) true))
  (:`Released`
    (set `self.Is RM Down` false)
    (`self.ShowMouseCursor`)
    (`self.SetDirectorInputMode`)
    (`self.SetActorHiddenInGame` (`self.CurrentMarker`) false)))

(event `Key|A`
  (params (Key :type "Key Structure"))
  (:`Pressed`
    (set `self.Is Left Pressed` true))
  (:`Released`
    (set `self.Is Left Pressed` false)))

(event `Key|S`
  (params (Key :type "Key Structure"))
  (:`Pressed`
    (set `self.Is Backward Pressed` true))
  (:`Released`
    (set `self.Is Backward Pressed` false)))

(event `Key|MouseScrollUp`
  (params (Key :type "Key Structure"))
  (:`Pressed`
    (bind _returnvalue (`/Game/Architect/Architect/Gizmo/Blueprints/BP_Gizmo.IsGizmoAttached` (`self.Gizmo`) :!label _label))
    (if _returnvalue
      (bind _returnvalue_2 (`/Game/Architect/Architect/Gizmo/Blueprints/BP_Gizmo.GetGizmoMode` (`self.Gizmo`)))
      (switch `/Game/Architect/Architect/Gizmo/Blueprints/GizmoMode` _returnvalue_2
        (:`NewEnumerator0`
          (`/Game/Architect/Architect/Gizmo/Blueprints/BP_Gizmo.SetGizmoMode` (`self.Gizmo`) "NewEnumerator1"))
        (:`NewEnumerator1`
          (`/Game/Architect/Architect/Gizmo/Blueprints/BP_Gizmo.SetGizmoMode` (`self.Gizmo`) "NewEnumerator2"))
        (:`NewEnumerator2`
          (`/Game/Architect/Architect/Gizmo/Blueprints/BP_Gizmo.SetGizmoMode` (`self.Gizmo`) "NewEnumerator0"))))))

(event `Key|D` :consume false
  (params (Key :type "Key Structure"))
  (:`Pressed`
    (set `self.Is Right Pressed` true))
  (:`Released`
    (set `self.Is Right Pressed` false)))

(event `Key|MouseScrollDown`
  (params (Key :type "Key Structure"))
  (:`Pressed`
    (goto _label)))

(event `StartDirectorMode`
  (bind (_returnvalue_location _returnvalue_rotation) (`KismetMathLibrary.BreakTransform` (`self.GetTransform` (`Controller.K2_GetPawn` (`self.Player`)))))
  (if (not (`self.IsModeActive`))
    (set `self.IsModeActive` true)
    (`self.K2_SetActorLocationAndRotation` (+ _returnvalue_location (0.0 0.0 100.0)) _returnvalue_rotation)
    (`PlayerController.SetViewTargetWithBlend` (`self.Player`) self 0.0 "VTBlend_Linear" 0.0 false)
    (`self.DisableInput` (`Controller.K2_GetPawn` (`self.Player`)) (`self.Player`)) ; Disable chars input
    (`self.EnableInput` (`self.Player`))
    (`self.ShowMouseCursor`)
    (`self.SetDirectorInputMode`)
    (`self.EnableSkylight`)
    (bind _returnvalue (`self.SpawnGizmo`))
    (bind _output_get (set `self.Gizmo` _returnvalue))
    (`self.SetActorHiddenInGame` _output_get true)
    (add `/Game/Architect/Architect/Gizmo/Blueprints/BP_Gizmo.OnInteractionStart` _output_get (delegate `GizmoStart`))
    (add `/Game/Architect/Architect/Gizmo/Blueprints/BP_Gizmo.OnInteractionEnd` _output_get (delegate `GizmoEnd`))
    (`self.AddWidgetToViewport` (`self.Hud`))
    (switch `/Game/Architect/Architect/EArchitectEditMode` (`self.CurrentMode`)
      (:`NewEnumerator0`
        (`self.EquipMarker` (`self.CurrentDecoData`))))))

(event `Key|E`
  (params (Key :type "Key Structure"))
  (:`Pressed`
    (set `self.Is Up Pressed` true))
  (:`Released`
    (set `self.Is Up Pressed` false)))

(event `Key|Q`
  (params (Key :type "Key Structure"))
  (:`Pressed`
    (set `self.Is Down Pressed` true))
  (:`Released`
    (set `self.Is Down Pressed` false)))

(event `Key|LeftMouseButton` :consume false
  (params (Key :type "Key Structure"))
  (:`Pressed`
    (switch `/Game/Architect/Architect/EArchitectEditMode` (`self.CurrentMode`)
      (:`NewEnumerator0`
        (`self.GetCursorWorldTransform`)
        (`self.ShowMouseCursor`)
        (`self.SetDirectorInputMode`)
        (`self.PlaceDecoration`))
      (:`NewEnumerator1`
        (bind (_location _rotation _hitactor) (`self.GetCursorWorldTransform`))
        (set `self.RecentHit` _hitactor)
        (`KismetSystemLibrary.Delay` 0.1)
        (if (not (`/Game/Architect/Architect/Gizmo/Blueprints/BP_Gizmo.IsInteractionInProgress` (`self.Gizmo`)))
          (`/Engine/EditorBlueprintResources/StandardMacros.IsValid` (`self.RecentHit`)
            (:`Is Valid`
              (bind _asdecoration_base (cast `/Game/Architect/Decorations/Decoration_Base` (`self.RecentHit`))
                (:`then`
                  (`self.SelectDecoration` _asdecoration_base))
                (:`CastFailed`
                  (if (not (== (`self.RecentHit`) (`self.Gizmo`))) :!label _label_2
                    (`self.UnselectDecoration`)))))
            (:`Is Not Valid`
              (goto _label_2))))))))

(event `GizmoStart`)

(event `GizmoEnd`
  (`self.DecorationMoved`))

(event `Key|Z`
  (params (Key :type "Key Structure"))
  (:`Pressed`
    (set `self.Is Z Pressed` true))
  (:`Released`
    (set `self.Is Z Pressed` false)))

(event `Key|Alt+A`
  (params (Key :type "Key Structure"))
  (:`Pressed`
    (if (`self.IsModeActive`)
      (if (`self.IsModeActive`) :!label _label_3
        (`self.DisableInput` (`self.Player`))
        (`PlayerController.SetViewTargetWithBlend` (`self.Player`) (`Controller.K2_GetPawn` (`self.Player`)) 0.0 "VTBlend_Linear" 0.0 false)
        (`self.EnableInput` (`Controller.K2_GetPawn` (`self.Player`)) (`self.Player`)) ; Enable chars input
        (set `self.IsModeActive` false)
        (`self.HideMouseCursor`)
        (`WidgetBlueprintLibrary.SetInputMode_GameOnly` (`self.Player`))
        (`self.UnselectDecoration`)
        (`self.ClearMarker`)
        (`self.DisableSkylight`)
        (`self.DestroyGizmo`)
        (`Widget.RemoveFromParent` (`self.Hud`))))))

(event `Key|C`
  (params (Key :type "Key Structure"))
  (:`Pressed`
    (set `self.Is C Pressed` true))
  (:`Released`
    (set `self.Is C Pressed` false)))

(event `StopDirectorMode`
  (goto _label_3))

(event `Key|LeftShift`
  (params (Key :type "Key Structure"))
  (:`Pressed`
    (set `self.Movement Rate` 100.0))
  (:`Released`
    (set `self.Movement Rate` 20.0)))

(event `Key|T`
  (params (Key :type "Key Structure"))
  (bind _gizmo (`self.Gizmo`))
  (:`Pressed`
    (bind _returnvalue (`/Game/Architect/Architect/Gizmo/Blueprints/BP_Gizmo.IsGizmoAttached` (`self.Gizmo`)))
    (if _returnvalue
      (bind _coordinatesystem (`/Game/Architect/Architect/Gizmo/Blueprints/BP_Gizmo.GetCoordinateSystem` (`self.Gizmo`)))
      (switch `/Game/Architect/Architect/Gizmo/Blueprints/GizmoCoordinateSystem` _coordinatesystem
        (:`NewEnumerator0`
          (`/Game/Architect/Architect/Gizmo/Blueprints/BP_Gizmo.SetCoordinateSystem` _gizmo "NewEnumerator1"))
        (:`NewEnumerator1`
          (`/Game/Architect/Architect/Gizmo/Blueprints/BP_Gizmo.SetCoordinateSystem` _gizmo "NewEnumerator0"))))))

(event `Key|M`
  (params (Key :type "Key Structure"))
  (:`Pressed`
    (switch `/Game/Architect/Architect/EArchitectEditMode` (`self.CurrentMode`)
      (:`NewEnumerator2`
        (`self.ChangeMode` "NewEnumerator0"))
      (:`NewEnumerator0`
        (`self.ChangeMode` "NewEnumerator1"))
      (:`NewEnumerator1`
        (`self.ChangeMode` "NewEnumerator0")))))

(event `Key|Delete`
  (params (Key :type "Key Structure"))
  (:`Pressed`
    (`self.DeleteDecoration` (`self.SelectedDecoration`))))

(event `self.ReceiveTick`
  (params (DeltaSeconds :type "Float (single-precision)"))
  (bind _returnvalue (`self.K2_GetActorLocation`))
  (bind _returnvalue_2 (`self.K2_GetActorRotation`))
  (bind (_returnvalue_roll _returnvalue_pitch _returnvalue_yaw) (`KismetMathLibrary.BreakRotator` (`self.K2_GetActorRotation`)))
  (bind (_deltax _deltay) (`PlayerController.GetInputMouseDelta` (`self.Player`)))
  (bind (_returnvalue_roll_2 _returnvalue_pitch_2 _returnvalue_yaw_2) (`KismetMathLibrary.BreakRotator` (`KismetMathLibrary.MakeRotator` 0.0 (* _deltay (`self.View Speed Y`)) (* _deltax (`self.View Speed X`)))))
  (bind _currentmarker (`self.CurrentMarker`)
    (:`then`
      (bind (_location _rotation) (`self.GetCursorWorldTransform`))
      (`self.K2_SetActorTransform` _currentmarker (`KismetMathLibrary.MakeTransform` _location _rotation (`self.GetActorScale3D`)) false false))
    (:`else`
      _))
  (`|ExecutionSequence`
    (:`then_0`
      (if (`self.Is Forward Pressed`)
        (set `self.Forward Velocity` 1.0)
        (elif (`self.Is Backward Pressed`)
          (set `self.Forward Velocity` -1.0)
          (else
            (set `self.Forward Velocity` 0.0)))))
    (:`then_1`
      (if (`self.Is Right Pressed`)
        (set `self.Right Velocity` 1.0)
        (elif (`self.Is Left Pressed`)
          (set `self.Right Velocity` -1.0)
          (else
            (set `self.Right Velocity` 0.0)))))
    (:`then_2`
      (if (`self.Is Up Pressed`)
        (set `self.Up Velocity` 1.0)
        (elif (`self.Is Down Pressed`)
          (set `self.Up Velocity` -1.0)
          (else
            (set `self.Up Velocity` 0.0)))))
    (:`then_3`
      (`self.K2_SetActorLocation` (`KismetMathLibrary.VInterpTo` _returnvalue (+ _returnvalue (* (+ (* (`KismetMathLibrary.GetForwardVector` _returnvalue_2) (`self.Forward Velocity`)) (* (`KismetMathLibrary.GetRightVector` _returnvalue_2) (`self.Right Velocity`)) (* (`KismetMathLibrary.GetUpVector` _returnvalue_2) (`self.Up Velocity`))) (`self.Movement Rate`))) DeltaSeconds (`self.Movement Accel`)))
      (if (`self.Is RM Down`)
        (`self.K2_AddActorLocalRotation` (`KismetMathLibrary.MakeRotator` 0.0 _returnvalue_pitch_2 _returnvalue_yaw_2))
        (`self.K2_SetActorRotation` (`KismetMathLibrary.MakeRotator` 0.0 (`KismetMathLibrary.FClamp` _returnvalue_pitch -80.0 80.0) _returnvalue_yaw))))))

(event `SelectDecoration`
  (params (Decoration :type "/Game/Architect/Decorations/Decoration_Base Object Reference"))
  (bind _output_get (set `self.SelectedDecoration` Decoration))
  (`/Game/Architect/Architect/Gizmo/Blueprints/BP_Gizmo.AttachGizmo` (`self.Gizmo`) _output_get)
  (`self.SetActorHiddenInGame` (`self.Gizmo`) false)
  (`/Game/Architect/Decorations/Decoration_Base.StartEditing` _output_get self))

(event `UnselectDecoration`
  (`self.SetActorHiddenInGame` (`self.Gizmo`) true)
  (`/Game/Architect/Decorations/Decoration_Base.StopEditing` (`self.SelectedDecoration`))
  (set `self.SelectedDecoration` null))

(event `DeleteDecoration`
  (params (Decoration :type "/Game/Architect/Decorations/Decoration_Base Object Reference"))
  (`/Engine/EditorBlueprintResources/StandardMacros.IsValid` Decoration
    (:`Is Valid`
      (set `self.PendingDelete` Decoration)
      (`self.UnselectDecoration`)
      (`/Game/Architect/Decorations/Decoration_Base.Delete` (`self.PendingDelete`)))))

(event `PlaceDecoration`
  (`self.ShowMouseCursor`)
  (bind _currentmarker (`self.CurrentMarker`)
    (:`then`
      (`/Game/Architect/Decorations/Markers/Marker_Base.Place` _currentmarker (`self.ArchitectMod`)))
    (:`else`)))

(event `DecorationMoved`
  (bind _selecteddecoration (`self.SelectedDecoration`)
    (:`then`
      (`/Game/Architect/Decorations/Decoration_Base.TransformChanged` _selecteddecoration true))
    (:`else`)))

(event `ChangeMode`
  (params (CurrentMode :type "/Game/Architect/Architect/EArchitectEditMode Enum" :default "NewEnumerator0"))
  (bind _output_get (set `self.CurrentMode` CurrentMode))
  (`/Game/Architect/Architect/HUD/ArchtectHud.SetEditMode` (`self.Hud`) _output_get)
  (switch `/Game/Architect/Architect/EArchitectEditMode` _output_get
    (:`NewEnumerator0`
      (`self.SetDecorationSelectorsVisible` true)
      (`self.UnselectDecoration`)
      (`self.CurrentMarker`
        (:`then`)
        (:`else`
          (`self.EquipMarker` (`self.CurrentDecoData`)))))
    (:`NewEnumerator1`
      (`self.SetDecorationSelectorsVisible` false)
      (`self.ClearMarker`))))

(event `Key|Ctrl+D` :consume false
  (params (Key :type "Key Structure"))
  (:`Pressed`
    (switch `/Game/Architect/Architect/EArchitectEditMode` (`self.CurrentMode`)
      (:`NewEnumerator1`
        (bind _selecteddecoration (`self.SelectedDecoration`)
          (:`then`
            (`/Game/Architect/Decorations/Decoration_Base.Duplicate` _selecteddecoration)
            (`self.SetDecorationSelectorsVisible` false))
          (:`else`))))))

(fn `ClearEditorWidget`
  (bind _hud (`self.Hud`)
    (:`then`
      (`/Game/Architect/Architect/HUD/ArchtectHud.ClearEditorWidget` _hud))
    (:`else`)))

(fn `ClearMarker`
  (bind _currentmarker (`self.CurrentMarker`)
    (:`then`
      (`self.K2_DestroyActor` _currentmarker)
      (set `self.CurrentMarker` null))
    (:`else`)))

(fn `DestroyGizmo`
  (bind _gizmo (`self.Gizmo`)
    (:`then`
      (`self.K2_DestroyActor` _gizmo)
      (set `self.Gizmo` null))
    (:`else`)))

(fn `DisableSkylight`
  (`SceneComponent.SetVisibility` (`self.SkyLight`) false false))

(fn `EnableSkylight`
  (`SceneComponent.SetVisibility` (`self.SkyLight`) true false))

(fn `EquipMarker`
  (params (DecoData :type "/Game/Architect/Decorations/DecorationData Structure"))
  (returns (ReturnValue :type Boolean))
  (set `self.CurrentDecoData` DecoData)
  (`self.ClearMarker`)
  (if (and (`|EnumEquality` (`self.CurrentMode`) "NewEnumerator0") (`self.IsModeActive`))
    (bind _returnvalue (`|SpawnActorFromClass` (`.MarkerClass_8_799FDF3A46F6488740D0D49EE2D1BE05` (break `/Game/Architect/Decorations/DecorationData` (`self.CurrentDecoData`))) (`KismetMathLibrary.MakeTransform` (0.0 0.0 0.0)) "AlwaysSpawn" "OverrideRootScale" null null))
    (bind _output_get (set `self.CurrentMarker` _returnvalue))
    (`/Game/Architect/Decorations/Markers/Marker_Base.LoadFromData` _output_get (`self.CurrentDecoData`))
    (return true)
    (else
      (return true))))

(fn `GetCursorWorldTransform`
  (returns (Location :type "Vector Structure") (Rotation :type "Rotator Structure") (HitActor :type "Actor Object Reference"))
  (bind (_worldlocation _worlddirection) (`PlayerController.DeprojectMousePositionToWorld` (`self.Player`)))
  (bind (_segmentstart _segmentend) (`/Game/Architect/Libraries/ArchitectFunctions.LineSegmentFromDirection` _worldlocation _worlddirection 100000.0))
  (bind (_outhit _returnvalue) (`KismetSystemLibrary.LineTraceSingle` _segmentstart _segmentend "TraceTypeQuery1" true (`|MakeArray` null null (`self.SelectedDecoration`) :!type "Actor Object Reference")))
  (if _returnvalue
    (bind (_bblockinghit _binitialoverlap _time _distance _location _impactpoint _normal _impactnormal _physmat _hitactor) (`GameplayStatics.BreakHitResult` _outhit))
    (return _location (`KismetMathLibrary.MakeRotFromZ` _normal) _hitactor)))

(fn `SetDecorationSelectorsVisible`
  (params (NewHidden :type Boolean))
  (bind _outactors (`GameplayStatics.GetAllActorsOfClass` "/Game/Architect/Decorations/Decoration_Base.Decoration_Base_C"))
  (for _array_element _outactors
    (`/Game/Architect/Decorations/Decoration_Base.SetSelectorVisible` _array_element NewHidden)))

(fn `SetEditorWidget`
  (params (EditorWidget :type "/Game/Architect/Decorations/DecoEditorWidget_Base Object Reference"))
  (bind _hud (`self.Hud`)
    (:`then`
      (`/Game/Architect/Architect/HUD/ArchtectHud.SetEditorWidget` _hud EditorWidget))
    (:`else`)))

(fn `SpawnGizmo`
  (returns (ReturnValue :type "/Game/Architect/Architect/Gizmo/Blueprints/BP_Gizmo Object Reference"))
  (bind _returnvalue (`|SpawnActorFromClass` "/Game/Architect/Architect/Gizmo/Blueprints/BP_Gizmo.BP_Gizmo_C" (`KismetMathLibrary.MakeTransform` (0.0 0.0 0.0)) "AlwaysSpawn" "OverrideRootScale" null null))
  (return _returnvalue))

(fn `UserConstructionScript`)